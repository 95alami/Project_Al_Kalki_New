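; Sinker is an enemy character that continually chases the player and picks attacks by distance.
; AIMoveTo reissues every 0.2 seconds, while a looping one-second timer checks range unless IsAttacking is set.
; Near triggers a random attack, anticipate or dodge montage, with a delay on its length clearing the flag.
; Mid only prints; far prints a random label and replays the current AttMontage without choosing one.
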(event `self.ReceiveBeginPlay`
  ;[1 1 1] Initialize
  (set `self.Alive` true)
  (`KismetSystemLibrary.Delay` 0.2)
  (`self.SeekPlayer`)
  (`self.DistancePlayer`))

(event `DistancePlayer`
  ;[1 1 1] Player Distance Function
  (`KismetSystemLibrary.K2_SetTimer` null "PlayerDistance" 1.0 true))

(event `SeekPlayer`
  ;[1 1 1] Seek Player Loop
  (`|AIMoveTo` self (0.0 0.0 0.0) (`GameplayStatics.GetPlayerCharacter` 0) 200.0
    (:`then`
      _)
    (:`OnSuccess`
      _)
    (:`OnFail`
      _))
  (`KismetSystemLibrary.Delay` 0.2)
  (`self.SeekPlayer`))

(event `Close Range`
  ;[1 1 1] Close Attack
  (set `self.IsAttacking` true)
  (switch `int` (`KismetMathLibrary.RandomIntegerInRange` 0 2)
    (:`0`
      (`KismetSystemLibrary.PrintString` "Attack" true true (struct :`G` 0.2376 :`B` 0.36 :`A` 1.0))
      (set `self.AttMontage` "/Game/Sinker/Montage/Sinker_Att.Sinker_Att"))
    (:`1`
      (`KismetSystemLibrary.PrintString` "Anticipate" true true (struct :`G` 0.2376 :`B` 0.36 :`A` 1.0))
      (set `self.AttMontage` "/Game/Sinker/Montage/Sinker_Anticipate.Sinker_Anticipate"))
    (:`2`
      (`KismetSystemLibrary.PrintString` "Dodge" true true (struct :`G` 0.2376 :`B` 0.36 :`A` 1.0))
      (set `self.AttMontage` "/Game/Sinker/Montage/Sinker_Doge.Sinker_Doge")))
  (bind _returnvalue (`self.PlayAnimMontage` (`self.AttMontage`)))
  (`KismetSystemLibrary.Delay` _returnvalue)
  (set `self.IsAttacking` false))

(event `Long Range`
  ;[1 1 1] Far Attack
  (set `self.IsAttacking` true)
  (switch `int` (`KismetMathLibrary.RandomIntegerInRange` 0 2)
    (:`0`
      (`KismetSystemLibrary.PrintString` "S1" true true (struct :`R` 0.18 :`B` 0.010301 :`A` 1.0)))
    (:`1`
      (`KismetSystemLibrary.PrintString` "S2" true true (struct :`R` 0.18 :`B` 0.010301 :`A` 1.0)))
    (:`2`
      (`KismetSystemLibrary.PrintString` "S3" true true (struct :`R` 0.18 :`B` 0.010301 :`A` 1.0))))
  (bind _returnvalue (`self.PlayAnimMontage` (`self.AttMontage`)))
  (`KismetSystemLibrary.Delay` _returnvalue)
  (set `self.IsAttacking` false))

(fn `PlayerDistance`
  (if (not (`self.IsAttacking`))
    ;[1 1 1] Detect Player Distance
    (bind _output_get (set `self.Distance` (`KismetMathLibrary.VSize` (- (`self.K2_GetActorLocation`) (`self.K2_GetActorLocation` (`GameplayStatics.GetPlayerCharacter` 0))))))
    ;[1 1 1] Mid Range
    (if (and (>= _output_get 301.0) (<= _output_get 600.0))
      (`KismetSystemLibrary.PrintString` "MID" true true (struct :`R` 0.76 :`G` 0.245537 :`A` 1.0))
      (else
        ;[1 1 1] Far Range
        (if (>= _output_get 601.0)
          (`KismetSystemLibrary.PrintString` "FAR" true true (struct :`R` 0.275 :`G` 0.017043 :`B` 0.014307 :`A` 1.0))
          (`self.Long Range`)
          (else
            ;[1 1 1] Close Range
            (if (<= _output_get 300.0)
              _
              (else
                _))
            (`KismetSystemLibrary.PrintString` "NEAR")
            (`self.Close Range`)))))))

(fn `UserConstructionScript`)