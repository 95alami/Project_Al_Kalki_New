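; Shooter enemy AI character that chases the player and picks randomized attacks based on range.
; A recursive seek loop uses AI MoveTo, while a looping timer measures distance and triggers close, mid or long range events.
; Each event plays a random push, dodge, shoot or run montage, then resumes seeking when it ends.
; BulletShoot spawns a bullet from the RHS component aimed at the player, though nothing in this graph calls it.
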(event `self.ReceiveBeginPlay`
  ;[1 1 1] Initialize
  (set `self.Alive` true)
  (`KismetSystemLibrary.Delay` 0.2)
  (`self.SeekPlayer`)
  (`self.DistancePlayer`))

(event `DistancePlayer`
  ;[1 1 1] Player Distance Function
  (`KismetSystemLibrary.K2_SetTimer` null "PlayerDistance" 1.0 true))

(event `SeekPlayer`
  ;[1 1 1] Seek Player Loop
  (if (`self.IsAttacking`)
    (`MovementComponent.StopMovementImmediately` (`self.CharacterMovement`))
    (else
      (`|AIMoveTo` self (0.0 0.0 0.0) (`GameplayStatics.GetPlayerCharacter` 0) 200.0
        (:`then`
          _)
        (:`OnSuccess`
          _)
        (:`OnFail`
          _))
      (`KismetSystemLibrary.Delay` 0.2)
      (`self.SeekPlayer`))))

(event `Close Range`
  ;[1 1 1] Attack Close
  (set `self.IsAttacking` true)
  (switch `int` (`KismetMathLibrary.RandomIntegerInRange` 0 1)
    (:`0`
      (`KismetSystemLibrary.PrintString` "Push" true true (struct :`R` 0.05 :`G` 0.05 :`B` 0.05 :`A` 1.0))
      (set `self.AttMontage` "/Game/Jakel/Animations/Push.Push"))
    (:`1`
      (`KismetSystemLibrary.PrintString` "Dodge" true true (struct :`R` 0.05 :`G` 0.05 :`B` 0.05 :`A` 1.0))
      (set `self.AttMontage` "/Game/Jakel/Animations/Stand.Stand")))
  (bind _returnvalue (`self.PlayAnimMontage` (`self.AttMontage`)))
  (`KismetSystemLibrary.Delay` _returnvalue)
  (set `self.IsAttacking` false)
  (`self.SeekPlayer`))

(event `BulletShoot`
  (bind _returnvalue (`SceneComponent.K2_GetComponentLocation` (`self.R_H_S`)))
  ;[1 1 1] Shoot Bullet
  (`|SpawnActorFromClass` "/Game/Jakel/Bullet_BP.Bullet_BP_C" (`KismetMathLibrary.MakeTransform` _returnvalue (`KismetMathLibrary.FindLookAtRotation` _returnvalue (`self.K2_GetActorLocation` (`GameplayStatics.GetPlayerCharacter` 0)))) "Undefined" "OverrideRootScale"))

(event `Mid Range`
  ;[1 1 1] Attack Mid
  (set `self.IsAttacking` true)
  (switch `int` (`KismetMathLibrary.RandomIntegerInRange` 0 2)
    (:`0`
      (`KismetSystemLibrary.PrintString` "Shoot" true true (struct :`R` 0.05 :`G` 0.05 :`B` 0.05 :`A` 1.0))
      (set `self.AttMontage` "/Game/Jakel/Animations/Shooting.Shooting"))
    (:`1`
      (`KismetSystemLibrary.PrintString` "Dodge" true true (struct :`R` 0.045 :`G` 0.045 :`B` 0.045 :`A` 1.0))
      (set `self.AttMontage` "/Game/Jakel/Animations/Stand.Stand"))
    (:`2`
      (`KismetSystemLibrary.PrintString` "Anticipate" true true (struct :`R` 0.04 :`G` 0.04 :`B` 0.04 :`A` 1.0))
      (set `self.AttMontage` "/Game/Jakel/Animations/Shooting.Shooting")))
  (bind _returnvalue (`self.PlayAnimMontage` (`self.AttMontage`)))
  (`KismetSystemLibrary.Delay` _returnvalue)
  (set `self.IsAttacking` false)
  (`self.SeekPlayer`))

(event `Long Range`
  ;[1 1 1] Attack Far
  (set `self.IsAttacking` true)
  (switch `int` (`KismetMathLibrary.RandomIntegerInRange` 0 2)
    (:`0`
      (`KismetSystemLibrary.PrintString` "Shoot" true true (struct :`R` 0.05 :`G` 0.05 :`B` 0.05 :`A` 1.0))
      (set `self.AttMontage` "/Game/Jakel/Animations/Shooting.Shooting"))
    (:`1`
      (`KismetSystemLibrary.PrintString` "Run" true true (struct :`R` 0.045 :`G` 0.045 :`B` 0.045 :`A` 1.0))
      (set `self.AttMontage` "/Game/Jakel/Run.Run"))
    (:`2`
      (`KismetSystemLibrary.PrintString` "Run2" true true (struct :`R` 0.045 :`G` 0.045 :`B` 0.045 :`A` 1.0))
      (set `self.AttMontage` "/Game/Jakel/Run.Run")))
  (bind _returnvalue (`self.PlayAnimMontage` (`self.AttMontage`)))
  (`KismetSystemLibrary.Delay` _returnvalue)
  (set `self.IsAttacking` false)
  (`self.SeekPlayer`))

(fn `PlayerDistance`
  (if (not (`self.IsAttacking`))
    ;[1 1 1] Detect Player Distance
    (bind _output_get (set `self.Distance` (`KismetMathLibrary.VSize` (- (`self.K2_GetActorLocation`) (`self.K2_GetActorLocation` (`GameplayStatics.GetPlayerCharacter` 0))))))
    ;[1 1 1] Mid Range
    (if (and (>= _output_get 251.0) (<= _output_get 500.0))
      (`KismetSystemLibrary.PrintString` "MID" true true (struct :`R` 0.125 :`G` 0.125 :`B` 0.125 :`A` 1.0))
      (`self.Mid Range`)
      (else
        ;[1 1 1] Far Range
        (if (>= _output_get 501.0)
          (`KismetSystemLibrary.PrintString` "FAR" true true (struct :`R` 0.095 :`G` 0.095 :`B` 0.095 :`A` 1.0))
          (`self.Long Range`)
          (else
            ;[1 1 1] Close Range
            (if (<= _output_get 250.0)
              _
              (else
                _))
            (`KismetSystemLibrary.PrintString` "NEAR" true true (struct :`R` 0.155 :`G` 0.155 :`B` 0.155 :`A` 1.0))
            (`self.Close Range`)))))))

(fn `UserConstructionScript`)